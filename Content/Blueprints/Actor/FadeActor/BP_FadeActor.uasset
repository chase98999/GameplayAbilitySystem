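; BP_FadeActor is an actor that shows its mesh partially faded at runtime through a "Fade" material parameter.
; The construction script creates a dynamic material instance from each of the mesh's materials and stores them in an array.
; BeginPlay assigns those instances to the matching mesh slots, then sets Fade to a fixed halfway value on each, with no animation over time.
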(event `self.ReceiveBeginPlay`
  (`self.SetMaterialsToDynamicInstances`)
  (for _array_element (`self.DynamicMaterialInstances`)
    (`MaterialInstanceDynamic.SetScalarParameterValue` _array_element "Fade" 0.5)))

(fn `SetMaterialsToDynamicInstances`
  (for (_array_element _array_index) (`self.DynamicMaterialInstances`)
    (`PrimitiveComponent.SetMaterial` (`self.Mesh`) _array_index _array_element)))

(fn `UserConstructionScript`
  (`KismetArrayLibrary.Array_Clear` (`self.DynamicMaterialInstances`))
  (bind _output_get (set `self.OriginalMaterials` (`MeshComponent.GetMaterials` (`self.Mesh`))))
  (for _array_element _output_get
    (bind _returnvalue (`KismetMaterialLibrary.CreateDynamicMaterialInstance` _array_element))
    (`KismetArrayLibrary.Array_AddUnique` (`self.DynamicMaterialInstances`) _returnvalue)))