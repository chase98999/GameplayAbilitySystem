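; GA_FireBolt is Aura's Fire Bolt gameplay ability, which casts a projectile at the target under the mouse.
; It takes mouse target data, aiming at a hit character's location or otherwise the hit point, and turns the avatar to face it.
; The cast montage plays, and its gameplay event triggers SpawnProjectile from the weapon socket, ending the ability after a short delay.
; The CommitAbility result only feeds a debug print, so a failed commit does not stop the cast.
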(event `self.K2_ActivateAbility`
  (bind _returnvalue (`self.K2_CommitAbility`))
  (`KismetSystemLibrary.PrintString` "true" _returnvalue)
  (bind (_asynctaskproxy _datahandle) (`TargetDataUnderMouse.CreateTargetDataUnderMouse`)
    (:`ValidData`
      (`self.DetermineProjectileTargetLocation` _datahandle)
      (`AbilityTask_PlayMontageAndWait.CreatePlayMontageAndWaitProxy` "None" "/Game/Assets/Characters/Aura/Animations/Abilities/AM_Cast_FireBolt.AM_Cast_FireBolt"
        (:`then`
          (`AbilityTask_WaitGameplayEvent.WaitGameplayEvent` (struct :`TagName` "Event.Montage.FireBolt") null
            (:`EventReceived`
              (`self.SpawnProjectile` (`self.ProjectileTargetLocation`) (`BlueprintGameplayTagLibrary.MakeLiteralGameplayTag` (struct :`TagName` "CombatSocket.Weapon")))
              (`KismetSystemLibrary.Delay` 0.5)
              (`self.K2_EndAbility`))))))))

(fn `DetermineProjectileTargetLocation`
  (params (HitResult :type "GameplayAbilityTargetDataHandle Structure (by ref)"))
  (bind (_bblockinghit _binitialoverlap _time _distance _location _impactpoint _normal _impactnormal _physmat _hitactor) (`GameplayStatics.BreakHitResult` (`AbilitySystemBlueprintLibrary.GetHitResultFromTargetData` HitResult)))
  (cast `AuraCharacterBase` _hitactor
    (:`then`
      (set `self.ProjectileTargetLocation` (`Actor.K2_GetActorLocation` _hitactor)))
    (:`CastFailed`
      (set `self.ProjectileTargetLocation` _location)))
  (message `CombatInterface.UpdateFacingTarget` (`self.GetAvatarActorFromActorInfo`) (`self.ProjectileTargetLocation`)))