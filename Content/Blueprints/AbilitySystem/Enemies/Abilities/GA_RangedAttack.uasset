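; Enemy gameplay ability for a ranged attack that fires a projectile at the avatar's combat target.
; On activation it turns the avatar toward the target, then plays a random attack montage from the avatar's list.
; A gameplay event matching the montage's tag triggers SpawnProjectile at the target's location at that moment.
; The ability ends when the montage completes or is interrupted or cancelled, or when no montage is available.
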(event `self.K2_ActivateAbility`
  (bind _returnvalue (`self.GetAvatarActorFromActorInfo`))
  (bind _returnvalue_2 (`self.GetAvatarActorFromActorInfo`))
  (bind _returnvalue_3 (message `EnemyInterface.GetCombatTarget` _returnvalue_2))
  (bind _ascombat_interface (cast `CombatInterface` _returnvalue_2))
  (`CombatInterface.UpdateFacingTarget` _ascombat_interface (`Actor.K2_GetActorLocation` _returnvalue_3))
  (bind _returnvalue_4 (message `CombatInterface.GetAttackMontages` (`self.GetAvatarActorFromActorInfo`)))
  (bind (_outitem _outindex) (`KismetArrayLibrary.Array_Random` _returnvalue_4))
  (bind _output_get (set `self.TaggedMontage` _outitem))
  (if (== _outindex -1)
    (`self.K2_EndAbility`)
    (else
      (bind (_montage _montagetag) (break `TaggedMontage` _output_get))
      (`AbilityTask_PlayMontageAndWait.CreatePlayMontageAndWaitProxy` "None" _montage 1.0 "None" false
        (:`then`
          (`AbilityTask_WaitGameplayEvent.WaitGameplayEvent` _montagetag null
            (:`EventReceived`
              (message `CombatInterface.GetCombatSocketLocation` _returnvalue _montagetag)
              (bind _returnvalue_5 (message `EnemyInterface.GetCombatTarget` _returnvalue))
              (`self.SpawnProjectile` (`Actor.K2_GetActorLocation` _returnvalue_5)))))
        (:`OnCompleted`
          (`self.K2_EndAbility` :!label _label))
        (:`OnInterrupted`
          (goto _label))
        (:`OnCancelled`
          (goto _label))))))